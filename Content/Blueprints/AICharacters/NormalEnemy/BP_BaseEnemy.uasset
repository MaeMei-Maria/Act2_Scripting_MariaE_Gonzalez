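; Base enemy character Blueprint that patrols, screams, strafes and makes melee attacks, exposing these actions as events and functions.
; Attack montage notifies trigger a sphere trace at the left hand socket to damage pawns, while the scream montage sets a ready flag on completion.
; Patrol points cycle along a path, and movement speed switches between idle, walk and attack presets.
; At zero health it plays a death animation, notifies BP_MyAIController and destroys itself.
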(event EventLaunchScream
  (Animation|Montage|PlayMontage (Variables|Character|GetMesh) "/Game/Mesh/Enemy/Animations/AnimMontage/AM_EnemyScream.AM_EnemyScream"
    (:OnCompleted
      (Variables|Default|SetIsReady true))))

(event EventSetStrafe
  (params (State :type Boolean))
  (Variables|Default|SetIsStrafing State))

(event Game|Damage|EventAnyDamage
  (params (Damage :type Float%20%28single-precision%29) (DamageType :type Damage%20Type%20Object%20Reference) (InstigatedBy :type Controller%20Object%20Reference) (DamageCauser :type Actor%20Object%20Reference))
  (bind _output_get (Variables|Default|SetHealth (- (Variables|Default|GetHealth) Damage)))
  (if (<= _output_get 0.0)
    (Components|Animation|PlayAnimation (Variables|Character|GetMesh) "/Game/Mesh/Enemy/Animations/Enemy_Death_Anim.Enemy_Death_Anim" false)
    (Default|OnDeath (.AsBP%20My%20AIController (Utilities|Casting|CastToBP_MyAIController (AI|GetAIController self))))
    (Utilities|FlowControl|Delay 2.0)
    (Actor|DestroyActor)))

(event EventLaunchAttack
  (Animation|Montage|PlayMontage (Variables|Character|GetMesh) "/Game/Mesh/Enemy/Animations/AnimMontage/AM_EnemyAttacking.AM_EnemyAttacking"
    (:OnNotifyBegin
      (CallFunction|MakeDamage))))

(fn ConstructionScript)

(fn MakeDamage
  (bind _mesh (Variables|Character|GetMesh))
  (bind _returnvalue (Transformation|GetSocketLocation _mesh "LeftHandSocket"))
  (bind (_outhit _returnvalue_2) (Collision|SphereTraceForObjects _returnvalue _returnvalue 4e+01 (Utilities|Array|MakeArray "ObjectTypeQuery3") false (Utilities|Array|MakeArray self) "ForDuration"))
  (if _returnvalue_2
    (Game|Damage|ApplyDamage (.HitActor (Collision|BreakHitResult _outhit)) 2e+01 0 0)))

(fn CalculateNewPatrolPoint
  (bind _output_get (Variables|Default|SetCurrentPoint (Default|GetLocationatIndex (Variables|Default|GetPatrolPath) (Variables|Default|GetCurrentIndex))))
  (Variables|Default|SetCurrentIndex (Math|Integer|%(Integer) (+ (Variables|Default|GetCurrentIndex) 1) (Default|GetPathLenght (Variables|Default|GetPatrolPath))))
  (return _output_get))

(fn SetNewSpeed
  (params (Input :type BPE_EnemySpeeds%20Enum :default "NewEnumerator2"))
  (Variables|/Script/Engine.CharacterMovementComponent|SetMaxWalkSpeed (Variables|Character|GetCharacterMovement) (Utilities|Select :Index Input :NewEnumerator2 0.0 :NewEnumerator0 2.5e+02 :NewEnumerator1 5e+02))
  (return 0.0))