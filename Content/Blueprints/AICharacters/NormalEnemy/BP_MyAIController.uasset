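; AI controller for normal enemies that runs the BT_Enemy behavior tree and drives its blackboard from perception.
; On begin play it sets the player as Target and an initial state, and refreshes the target whenever the game mode signals a player respawn.
; Seeing the player switches CurrentState, while lost sight, noises or damage store a PointOfInterest and switch to investigating.
; OnDeath stops the brain logic and clears focus.
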(event OnTargetPerceptionUpdated(AIPerception)
  (params (Actor :type Actor%20Object%20Reference) (Stimulus :type AI%20Stimulus%20Structure))
  (Utilities|FlowControl|Sequence
    (:then_0
      (bind (_result _stateofstimulus) (CallFunction|CanSenseSomething "/Script/AIModule.AISense_Sight" Stimulus))
      (if _result
        (if _stateofstimulus
          (Development|PrintString "Vi algo")
          (CallFunction|OnActorSeen Actor)
          (else
            (Development|PrintString "Ya no veo nada")
            (CallFunction|OnInvestigating (.StimulusLocation (Utilities|Struct|BreakAIStimulus Stimulus)) :!label _label)))))
    (:then_1
      (bind (_result_2 _stateofstimulus_2) (CallFunction|CanSenseSomething "/Script/AIModule.AISense_Hearing" Stimulus))
      (if _result_2
        (if _stateofstimulus_2
          (Development|PrintString "eSCUCHÉ algo")
          (goto _label))))
    (:then_2
      (bind (_result_3 _stateofstimulus_3) (CallFunction|CanSenseSomething "/Script/AIModule.AISense_Damage" Stimulus))
      (if _result_3
        (if _stateofstimulus_3
          (Development|PrintString "Me hicieron daño")
          (goto _label))))))

(event Custom|CE_SetTarget
  ;[0 0.7474 0.7708 0.5] Da valor al target y al enum
  (CallFunction|UpdateTarget))

(event EventBeginPlay
  ;[0 0.7474 0.7708 0.5] Da valor al target y al enum
  (EventDispatchers|BindEventtoOnPlayerRespawn (.AsBP%20My%20Game%20Mode (Utilities|Casting|CastToBP_MyGameMode (Game|GetGameMode))) (delegate Custom|CE_SetTarget))
  (AI|RunBehaviorTree "/Game/Blueprints/AICharacters/NormalEnemy/BT_Enemy.BT_Enemy")
  (CallFunction|UpdateTarget)
  (CallFunction|SetCurrentState (Utilities|Enum|LiteralenumBPE_States "NewEnumerator0")))

(fn ConstructionScript)

(fn SetCurrentState
  (params (EnumValue :type BPE_States%20Enum :default "NewEnumerator0"))
  (AI|Components|Blackboard|SetValueasEnum (AI|GetBlackboard 0) (Utilities|Name|MakeLiteralName "CurrentState") EnumValue))

(fn CanSenseSomething
  (params (SenseType :type Object%20Class%20Reference) (Stimulus :type AI%20Stimulus%20Structure))
  (bind _returnvalue (Class|AIPerceptionSystem|GetSenseClassforStimulus Stimulus))
  (return (== SenseType _returnvalue) (Utilities|Struct|BreakAIStimulus Stimulus)))

(fn OnActorSeen
  (params (ActorSeen :type Actor%20Object%20Reference))
  (if (== ActorSeen (Game|GetPlayerCharacter 0))
    (CallFunction|SetCurrentState "NewEnumerator1")))

(fn OnInvestigating
  (params (PointOfInterest :type Vector))
  (AI|Components|Blackboard|SetValueasVector (AI|GetBlackboard 0) (Utilities|Name|MakeLiteralName "PointOfInterest") PointOfInterest)
  (CallFunction|SetCurrentState "NewEnumerator2"))

(fn UpdateTarget
  (AI|Components|Blackboard|SetValueasObject (AI|GetBlackboard 0) (Utilities|Name|MakeLiteralName "Target") (Game|GetPlayerCharacter 0)))

(fn OnDeath
  (AI|Logic|StopLogic (Variables|Default|GetBrainComponent) "")
  (AI|ClearFocus))