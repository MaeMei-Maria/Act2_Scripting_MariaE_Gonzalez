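; AI controller that runs the BT_Enemy behavior tree for enemy characters.
; On BeginPlay it stores the player character as the Blackboard Target and sets the initial state to the first BPE_States value.
; SetCurrentState writes a given state enum into the CurrentState Blackboard key.
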(event EventBeginPlay
  ;[0 0.7474 0.7708 0.5] Da valor al target y al enum
  (AI|RunBehaviorTree "/Game/Blueprints/AICharacters/BT_Enemy.BT_Enemy")
  (AI|Components|Blackboard|SetValueasObject (AI|GetBlackboard 0) (Utilities|Name|MakeLiteralName "Target") (Game|GetPlayerCharacter 0))
  (CallFunction|SetCurrentState (Utilities|Enum|LiteralenumBPE_States "NewEnumerator0")))

(fn ConstructionScript)

(fn SetCurrentState
  (params (EnumValue :type Byte))
  (AI|Components|Blackboard|SetValueasEnum (AI|GetBlackboard 0) (Utilities|Name|MakeLiteralName "CurrentState") EnumValue))