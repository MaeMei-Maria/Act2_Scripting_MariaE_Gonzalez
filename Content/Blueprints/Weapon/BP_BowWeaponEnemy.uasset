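; BP_BowWeaponEnemy is an enemy bow weapon that fires an instant hitscan shot at the player.
; Its CE_FireBow event plays the arrow sound at the world origin, leaving the EnemyLocation input unused.
; It then line-traces for Pawns from the bow's Sight socket to the player's location, offset by the player mesh's forward vector, and applies Damage to the hit actor.
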(event Custom|CE_FireBow
  (params (EnemyLocation :type Vector))
  (bind _returnvalue (Game|Player|GetPlayerPawn 0))
  (bind _asbp_player_character (Utilities|Casting|CastToBP_PlayerCharacter _returnvalue))
  (Audio|PlaySoundatLocation "/Game/SFX/Arrow/SC_Arrow.SC_Arrow" "0, 0, 0" "0, 0, 0" 1.0 1.0 0.0 0 0 0 0)
  (bind (_outhit _returnvalue_2) (Collision|LineTraceForObjects (Transformation|GetSocketLocation (Variables|Default|GetBow) "Sight") (+ (Transformation|GetActorLocation _asbp_player_character) (Math|Vector|GetForwardVector (Variables|/Script/Engine.Character|GetMesh _asbp_player_character))) (Utilities|Array|MakeArray "ObjectTypeQuery3") false 0 "None"))
  (if _returnvalue_2
    (Game|Damage|ApplyDamage (.HitActor (Collision|BreakHitResult _outhit)) (Variables|Default|GetDamage) 0 0)))

(fn ConstructionScript)