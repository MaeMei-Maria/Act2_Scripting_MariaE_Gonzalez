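; BP_SwordWeapon is a sword weapon Blueprint that damages pawns around the blade through a custom event, CE_SwordSphereTrace.
; The event runs a zero-length multi sphere trace at the Sword component's location, filtered to Pawn objects and drawn for debugging.
; It applies fixed damage to every hit actor.
; The ignore list holds the player controller, not its controlled pawn.
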(event Custom|CE_SwordSphereTrace
  (bind _sword (Variables|Default|GetSword))
  (bind _returnvalue (Transformation|GetWorldLocation _sword))
  (bind (_outhits _returnvalue_2) (Collision|MultiSphereTraceForObjects _returnvalue _returnvalue 4e+01 (Utilities|Array|MakeArray "ObjectTypeQuery3") false (Utilities|Array|MakeArray (.AsBP%20My%20Player%20Controller (Utilities|Casting|CastToBP_MyPlayerController (Game|GetPlayerController 0)))) "ForDuration"))
  (if _returnvalue_2
    (for _array_element _outhits
      (Game|Damage|ApplyDamage (.HitActor (Collision|BreakHitResult _array_element)) 25.0 0 0))))

(fn ConstructionScript)