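; BP_BowWeapon is a bow weapon that fires as an instant hitscan shot.
; CE_FireBow plays an arrow sound at the world origin, then runs a complex Visibility line trace forward from the bow's Sight socket out to Range, with debug drawing enabled.
; A hit applies Damage to the struck actor, followed by a short delay with nothing after it.
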(event Custom|CE_FireBow
  (bind _bow (Variables|Default|GetBow))
  (bind _returnvalue (Transformation|GetSocketLocation _bow "Sight"))
  (Audio|PlaySoundatLocation "/Game/SFX/Arrow/SC_Arrow.SC_Arrow" "0, 0, 0" "0, 0, 0" 1.0 1.0 0.0 0 0 0 0)
  (bind (_outhit _returnvalue_2) (Collision|LineTraceByChannel _returnvalue (+ _returnvalue (* (Math|Vector|GetForwardVector (Transformation|GetSocketRotation _bow "Sight")) (Variables|Default|GetRange))) "TraceTypeQuery1" true (Utilities|Array|MakeArray self) "ForDuration"))
  (if _returnvalue_2
    (Game|Damage|ApplyDamage (.HitActor (Collision|BreakHitResult _outhit)) (Variables|Default|GetDamage) 0 0)
    (Utilities|FlowControl|Delay 0.5)))

(fn ConstructionScript)