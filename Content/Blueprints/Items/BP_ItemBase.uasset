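; BP_ItemBase is a world item pickup that moves itself into the player's inventory on touch.
; On BeginPlay it loads its ItemData from DT_ItemData using ItemID as the row name and caches the player character.
; When the player overlaps its sphere, it adds ItemID and ItemQuantity through BPCInventorySystem.
; Only a successful add shows an inventory HUD notification and destroys the actor.
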(event OnComponentBeginOverlap(Sphere1)
  (params (OverlappedComponent :type Primitive%20Component%20Object%20Reference) (OtherActor :type Actor%20Object%20Reference) (OtherComp :type Primitive%20Component%20Object%20Reference) (OtherBodyIndex :type Integer) (bFromSweep :type Boolean) (SweepResult :type Hit%20Result%20Structure%20%28by%20ref%29))
  (bind _playercharacter (Variables|Default|GetPlayerCharacter))
  (if (== OtherActor _playercharacter)
    (bind _success (Default|AddItem (Variables|/Game/Blueprints/Player/BP_PlayerCharacter.BP_PlayerCharacter_C|GetBPC_InventorySystem _playercharacter) (Variables|Default|GetItemID) (Variables|Default|GetItemQuantity)))
    (if _success
      (Default|AddItemNotification (Variables|/Game/Blueprints/Player/BP_MyPlayerController.BP_MyPlayerController_C|GetInventoryHud (.AsBP%20My%20Player%20Controller (Utilities|Casting|CastToBP_MyPlayerController (Game|GetPlayerController 0)))) (Variables|Default|GetItemData) (Variables|Default|GetItemQuantity))
      (Actor|DestroyActor))))

(event EventBeginPlay
  (CallFunction|InizializeItemData)
  (Variables|Default|SetPlayerCharacter (.AsBP%20Player%20Character (Utilities|Casting|CastToBP_PlayerCharacter (Game|GetPlayerCharacter 0)))))

(fn ConstructionScript)

(fn InizializeItemData
  (bind _returnvalue (Utilities|GetDataTableRow "/Game/Blueprints/UI/Inventory/Components/DT_ItemData.DT_ItemData" (Utilities|String|StringToName (Variables|Default|GetItemID)))
    (:then
      (Variables|Default|SetItemData _returnvalue))))