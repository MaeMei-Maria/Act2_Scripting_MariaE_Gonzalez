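; Player controller that owns the player's health and arrow count and sets up input and the HUD.
; BeginPlay adds the input mapping, creates HUD, compass, inventory and hidden victory widgets, and binds bar resets to the game mode's respawn event.
; Damage, healing and arrow changes broadcast updates through dispatchers.
; At zero health it disables input, flags death on both linked anim graphs and destroys the character after a delay.
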(event Custom|CE_GetDamaged
  (params (Damage :type Float%20%28double-precision%29) (Anim :type AB%20Player%20Final%20Object%20Reference))
  ;[0.15 0.15 0.15 0.5] Resta la vida al player y activa la animación de morir
  (bind _output_get (Variables|Default|SetCurrentHealth (- (Variables|Default|GetCurrentHealth) Damage)))
  (Default|CallHealthUpdate (Variables|Default|GetCurrentHealth) (Variables|Default|GetMaxHealth))
  (if (<= _output_get 0.0)
    (Input|DisableInput (Game|Player|GetPlayerPawn 0) self)
    (Variables|/Game/Blueprints/Player/Animations/AB_Player.AB_Player_C|SetIsDeath (.AsAB%20Player (Utilities|Casting|CastToAB_Player (Class|AnimInstance|GetLinkedAnimGraphInstancebyTag Anim "NormalMove"))) true)
    (Variables|/Game/Blueprints/Player/Animations/AB_BowAnim.AB_BowAnim_C|SetIsDeath (.AsAB%20Bow%20Anim (Utilities|Casting|CastToAB_BowAnim (Class|AnimInstance|GetLinkedAnimGraphInstancebyTag Anim "StrafeMove"))) true)
    (Utilities|FlowControl|Delay 4.0)
    (Actor|DestroyActor (Game|GetPlayerCharacter 0))))

(event Custom|CE_SetBars
  (bind _maxhealth (Variables|Default|GetMaxHealth))
  ;[0.15 0.15 0.15 0.5] Setea la vida inicial, añade el mapping contex de los inputs y la interfaz
  (bind _output_get (Variables|Default|SetCurrentHealth _maxhealth))
  (Default|CallHealthUpdate _output_get _maxhealth)
  (bind _output_get_2 (Variables|Default|SetCurrentArrows 0))
  (Default|CallArrowsBarUpdate _output_get_2 (Variables|Default|GetMaxArrows)))

(event Custom|CE_WasteArrows
  (params (NumOfShot :type Integer))
  (bind _output_get (Variables|Default|SetCurrentArrows (- (Variables|Default|GetCurrentArrows) NumOfShot)))
  (Default|CallArrowsBarUpdate _output_get (Variables|Default|GetMaxArrows)))

(event EventBeginPlay
  (bind _returnvalue (PlayerController|LocalPlayerSubsystems|GetEnhancedInputLocalPlayerSubsystem))
  ;[0.15 0.15 0.15 0.5] Setea la vida inicial, añade el mapping contex de los inputs y la interfaz
  (CallFunction|CESetBars)
  (EventDispatchers|BindEventtoOnPlayerRespawn (.AsBP%20My%20Game%20Mode (Utilities|Casting|CastToBP_MyGameMode (Game|GetGameMode))) (delegate Custom|CE_SetBars))
  (Utilities|IsValid _returnvalue
    (:Is%20Valid
      (Input|AddMappingContext _returnvalue "/Game/Inputs/MyInputMapping.MyInputMapping" 0 "(bIgnoreAllPressedKeysUntilRelease=True,bForceImmediately=False,bNotifyUserSettings=False)")
      (CallFunction|AddHudComponents)
      (Default|ShowMessage (Variables|Default|GetPlayerMenu) "Reune 3 pares de engranajes para poder salir de aquí mediante el ascensor")
      (Default|CEInizialiteBar (Variables|Default|GetPlayerMenu) self))))

(fn ConstructionScript)

(fn AddHudComponents
  (Utilities|FlowControl|Sequence
    (:then_0
      (bind _returnvalue (UserInterface|CreateWidget "/Game/Blueprints/UI/WBP_PlayerHUD.WBP_PlayerHUD_C"))
      (bind _output_get (Variables|Default|SetPlayerMenu _returnvalue))
      (UserInterface|Viewport|AddtoViewport _output_get 0))
    (:then_1
      (bind _returnvalue_2 (UserInterface|CreateWidget "/Game/Blueprints/UI/Compass/WBP_CompassBar.WBP_CompassBar_C"))
      (UserInterface|Viewport|AddtoViewport _returnvalue_2 0))
    (:then_2
      (bind _returnvalue_3 (UserInterface|CreateWidget "/Game/Blueprints/UI/Inventory/WBP/WBP_InventoryHUD.WBP_InventoryHUD_C"))
      (bind _output_get_2 (Variables|Default|SetInventoryHud _returnvalue_3))
      (UserInterface|Viewport|AddtoViewport _output_get_2 1))
    (:then_3
      (bind _returnvalue_4 (UserInterface|CreateWidget "/Game/Blueprints/UI/WBP_Victory.WBP_Victory_C"))
      (bind _output_get_3 (Variables|Default|SetVictoryScreen _returnvalue_4))
      (UserInterface|Viewport|AddtoViewport _output_get_3 0)
      (Widget|SetVisibility (Variables|Default|GetVictoryScreen) "Hidden"))))

(fn HealPlayer
  (params (Amount :type Float%20%28double-precision%29))
  (if (not (>= (Variables|Default|GetCurrentHealth) (Variables|Default|GetMaxHealth)))
    (Audio|PlaySoundatLocation "/Game/SFX/Heal.Heal" (Transformation|GetActorLocation (Game|GetPlayerCharacter 0)) "0, 0, 0" 1.0 1.0 0.0 0 0 0 0)
    (bind _output_get (Variables|Default|SetCurrentHealth (+ Amount (Variables|Default|GetCurrentHealth))))
    (Default|CallHealthUpdate _output_get (Variables|Default|GetMaxHealth))))

(fn GetArrows
  (params (Amount :type Integer))
  (if (not (== (Variables|Default|GetCurrentArrows) (Variables|Default|GetMaxArrows)))
    (bind _output_get (Variables|Default|SetCurrentArrows (+ Amount (Variables|Default|GetCurrentArrows))))
    (Default|CallArrowsBarUpdate _output_get (Variables|Default|GetMaxArrows))))