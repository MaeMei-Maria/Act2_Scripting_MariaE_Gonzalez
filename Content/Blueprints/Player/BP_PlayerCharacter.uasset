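; Player character Blueprint that handles Enhanced Input for movement, looking, jumping, running, interaction and inventory slot scrolling.
; Movement follows control yaw, Run toggles max walk speed, and Jump also emits noise at the character's location.
; Interact passes the inventory component's valid look-at actor to its interact event.
; Scroll is meant to step the selected slot, but compares constant zero with zero, so neither branch changes it.
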(event Input|EnhancedActionEvents|EnhancedInputActionIA_Move
  (params (ActionValue :type Vector%202D%20Structure) (ElapsedSeconds :type Float%20%28double-precision%29) (TriggeredSeconds :type Float%20%28double-precision%29) (InputAction :type Input%20Action%20Object%20Reference :default "/Game/Inputs/IA_Move.IA_Move"))
  (bind _returnvalue (Pawn|GetControlRotation :!class /Script/Engine.Pawn))
  (Pawn|Input|AddMovementInput (Math|Vector|GetForwardVector (Math|Rotator|MakeRotator 0.0 0.0 (.yaw _returnvalue))) (.y ActionValue) false)
  (Pawn|Input|AddMovementInput (Math|Vector|GetRightVector (Math|Rotator|MakeRotator 0.0 0.0 (.yaw _returnvalue))) (.x ActionValue) false))

(event Input|EnhancedActionEvents|EnhancedInputActionIA_Look
  (params (ActionValue :type Vector%202D%20Structure) (ElapsedSeconds :type Float%20%28double-precision%29) (TriggeredSeconds :type Float%20%28double-precision%29) (InputAction :type Input%20Action%20Object%20Reference :default "/Game/Inputs/IA_Look.IA_Look"))
  (Pawn|Input|AddControllerYawInput (.x ActionValue))
  (Pawn|Input|AddControllerPitchInput (* (.y ActionValue) -1.0)))

(event Input|EnhancedActionEvents|EnhancedInputActionIA_Jump
  (params (ActionValue :type Boolean) (ElapsedSeconds :type Float%20%28double-precision%29) (TriggeredSeconds :type Float%20%28double-precision%29) (InputAction :type Input%20Action%20Object%20Reference :default "/Game/Inputs/IA_Jump.IA_Jump"))
  (Character|Jump)
  (Class|Actor|MakeNoise 1.0 0 (Transformation|GetActorLocation) 0.0 "None"))

(event Input|EnhancedActionEvents|EnhancedInputActionIA_Run
  (params (ActionValue :type Boolean) (ElapsedSeconds :type Float%20%28double-precision%29) (TriggeredSeconds :type Float%20%28double-precision%29) (InputAction :type Input%20Action%20Object%20Reference :default "/Game/Inputs/IA_Run.IA_Run"))
  (bind _charactermovement (Variables|Character|GetCharacterMovement))
  (:Triggered
    (Variables|/Script/Engine.CharacterMovementComponent|SetMaxWalkSpeed _charactermovement 6e+02))
  (:Completed
    (Variables|/Script/Engine.CharacterMovementComponent|SetMaxWalkSpeed _charactermovement 3e+02)))

(event Input|EnhancedActionEvents|EnhancedInputActionIA_Interact
  (params (ActionValue :type Boolean) (ElapsedSeconds :type Float%20%28double-precision%29) (TriggeredSeconds :type Float%20%28double-precision%29) (InputAction :type Input%20Action%20Object%20Reference :default "/Game/Inputs/IA_Interact.IA_Interact"))
  (bind _bp_inventorysystem (Variables|Default|GetBP_InventorySystem))
  (bind _lookatactor (Variables|/Game/Blueprints/UI/Inventory/Blueprint/BP_InventorySystem.BP_InventorySystem_C|GetLookAtActor _bp_inventorysystem)
    (:then
      (Default|CEPlayerInteract _bp_inventorysystem _lookatactor))
    (:else)))

(event Input|EnhancedActionEvents|EnhancedInputActionIA_ChangeItemScroll
  (params (ActionValue :type Float%20%28double-precision%29) (ElapsedSeconds :type Float%20%28double-precision%29) (TriggeredSeconds :type Float%20%28double-precision%29) (InputAction :type Input%20Action%20Object%20Reference :default "/Game/Inputs/IA_ChangeItemScroll.IA_ChangeItemScroll"))
  (bind _selectedslots (Variables|Slots|GetSelectedSlots))
  (bind _selectedslots_2 (Variables|Slots|GetSelectedSlots))
  ;[0.1142 0.15 0.09377 0.5] Slot del inventario selecionado
  (Math|Float|CompareFloat 0.0 0.0
    (:>
      (if (== _selectedslots_2 (Variables|Slots|GetMaxSlots))
        (Math|Integer|IncrementInt _selectedslots_2)))
    (:<
      (if (== _selectedslots 0)
        (Math|Integer|DecrementInt _selectedslots)))))

(event EventBeginPlay)

(fn ConstructionScript)